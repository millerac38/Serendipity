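; Beta player character Blueprint with movement along a single world axis, jumping, blocking and attacking through Enhanced Input.
; BeginPlay adds the IMC_move mapping context to the controlling player.
; Attack and block inputs set boolean state flags, with block changes ignored while attacking.
; Movement along world X and jump starts are suppressed only when both flags are true.
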(event `self.ReceiveBeginPlay`
  (bind _asplayer_controller (cast `PlayerController` (`self.GetController`)))
  (bind _returnvalue (pcsubsystem `EnhancedInputLocalPlayerSubsystem` _asplayer_controller))
  (`/Engine/EditorBlueprintResources/StandardMacros.IsValid` _returnvalue
    (:`Is Valid`
      (`EnhancedInputSubsystemInterface.AddMappingContext` _returnvalue "/Game/controls/IMC_move.IMC_move" 0 (struct)))))

(event `EnhancedInput|/Game/controls/IA_move`
  (params (ActionValue :type "Float (double-precision)") (ElapsedSeconds :type "Float (double-precision)") (TriggeredSeconds :type "Float (double-precision)") (InputAction :type "InputAction Object Reference" :default "/Game/controls/IA_move.IA_move"))
  (:`Triggered`
    (if (not (and (`self.isBlocking`) (`self.isAttacking`)))
      (`self.AddMovementInput` (1.0 0.0 0.0) (* ActionValue 2.0)))))

(event `EnhancedInput|/Game/controls/IA_Jump`
  (params (ActionValue :type "Float (double-precision)") (ElapsedSeconds :type "Float (double-precision)") (TriggeredSeconds :type "Float (double-precision)") (InputAction :type "InputAction Object Reference" :default "/Game/controls/IA_Jump.IA_Jump"))
  (:`Triggered`
    (if (not (and (`self.isBlocking`) (`self.isAttacking`)))
      (`self.Jump`)))
  (:`Canceled`
    (`self.StopJumping`)))

(event `EnhancedInput|/Game/controls/IA_block`
  (params (ActionValue :type Boolean) (ElapsedSeconds :type "Float (double-precision)") (TriggeredSeconds :type "Float (double-precision)") (InputAction :type "InputAction Object Reference" :default "/Game/controls/IA_block.IA_block"))
  (:`Triggered`
    (if (not (`self.isAttacking`))
      (set `self.isBlocking` true)))
  (:`Completed`
    (if (not (`self.isAttacking`))
      (set `self.isBlocking` false))))

(event `EnhancedInput|/Game/controls/IA_attack`
  (params (ActionValue :type Boolean) (ElapsedSeconds :type "Float (double-precision)") (TriggeredSeconds :type "Float (double-precision)") (InputAction :type "InputAction Object Reference" :default "/Game/controls/IA_attack.IA_attack"))
  (:`Triggered`
    (set `self.isAttacking` true))
  (:`Completed`
    (set `self.isAttacking` false)))

(fn `UserConstructionScript`)